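; BP_Water is a water collectible that shows a widget while the top-down character stands inside its sphere.
; Sphere overlap events toggle that widget and an overlap flag, which is named IsFoodOverlap despite this being water.
; OnCollected increments the character's WaterNumber, copies the count to NumOfWater in BP_GameInstance, then destroys the actor.
; Nothing in this graph calls OnCollected or reads the flag.
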(event `self.Sphere.OnComponentBeginOverlap`
  (params (OverlappedComponent :type "PrimitiveComponent Object Reference") (OtherActor :type "Actor Object Reference") (OtherComp :type "PrimitiveComponent Object Reference") (OtherBodyIndex :type Integer) (bFromSweep :type Boolean) (SweepResult :type "HitResult Structure (by ref)"))
  (cast `/Game/TopDown/Blueprints/BP_TopDownCharacter` OtherActor)
  (`SceneComponent.SetVisibility` (`self.Widget`) true false)
  (set `self.isFoodOverlap` true))

(event `self.Sphere.OnComponentEndOverlap`
  (params (OverlappedComponent :type "PrimitiveComponent Object Reference") (OtherActor :type "Actor Object Reference") (OtherComp :type "PrimitiveComponent Object Reference") (OtherBodyIndex :type Integer))
  (cast `/Game/TopDown/Blueprints/BP_TopDownCharacter` OtherActor)
  (`SceneComponent.SetVisibility` (`self.Widget`) false false)
  (set `self.isFoodOverlap` false))

(event `/Game/CollectSkill/BPI_Collectibles.OnCollected`
  (bind _returnvalue (`GameplayStatics.GetActorOfClass` "/Game/TopDown/Blueprints/BP_TopDownCharacter.BP_TopDownCharacter_C"))
  (bind _result (`/Engine/EditorBlueprintResources/StandardMacros.IncrementInt` (`/Game/TopDown/Blueprints/BP_TopDownCharacter.waterNumber` _returnvalue))
    (:`  `
      (bind _asbp_game_instance (cast `/Game/CollectSkill/BP_GameInstance` (`GameplayStatics.GetGameInstance`)))
      (set `/Game/CollectSkill/BP_GameInstance.NumOfWater` _result _asbp_game_instance)
      (`self.K2_DestroyActor`))))

(fn `UserConstructionScript`)